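; Player-drivable tank Blueprint that hands driving, aiming and firing to its TankMovement and TankAiming components.
; On BeginPlay it assigns track and turret meshes and the track physical material, then passes tracks, barrel and turret to those components.
; Movement axes forward intent to TankMovement, and Fire calls TankAiming.
; Aim axes rotate a separate azimuth gimbal (yaw) and spring arm (pitch), scaled by delta time, without directly turning the turret.
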(event `self.ReceiveBeginPlay`
  (`self.Setup Static Meshes`)
  (`TankAimingComponent.Initialise` (`self.TankAiming`) (`self.TankBarrel`) (`self.TankTurret`))
  (`TankMovementComponent.Initialise` (`self.TankMovement`) (`self.TankTrack Left`) (`self.TankTrack Right`)))

(event `InputAxis|MoveForward`
  (params (AxisValue :type "Float (single-precision)"))
  ;[1 1 1] Movement Input Binding
  (`TankMovementComponent.intendMoveForward` (`self.TankMovement`) AxisValue))

(event `InputAxis|Turn Right`
  (params (AxisValue :type "Float (single-precision)"))
  ;[1 1 1] Movement Input Binding
  (`TankMovementComponent.IntendTurnRight` (`self.TankMovement`) AxisValue))

(event `InputAxis|AimAzimuth`
  (params (AxisValue :type "Float (single-precision)"))
  ;[1 1 1] Aiming Input Binding
  ;;[1 1 1] AimAzimuth
  (`SceneComponent.K2_AddLocalRotation` (`self.Azimuth Gimbal`) (`KismetMathLibrary.MakeRotator` 0.0 0.0 (* AxisValue (`GameplayStatics.GetWorldDeltaSeconds`) 100.0)) false false))

(event `InputAxis|AimElevation`
  (params (AxisValue :type "Float (single-precision)"))
  ;[1 1 1] Aiming Input Binding
  ;;[1 1 1] AimElevation
  (`SceneComponent.K2_AddLocalRotation` (`self.SpringArm`) (`KismetMathLibrary.MakeRotator` 0.0 (* AxisValue (`GameplayStatics.GetWorldDeltaSeconds`) 100.0)) false false))

(event `InputAction|Fire`
  (params (Key :type "Key Structure"))
  ;[1 1 1] Aiming Input Binding
  ;;[1 1 1] Fire
  (:`Pressed`
    (`TankAimingComponent.Fire` (`self.TankAiming`))))

(fn `Setup Static Meshes`
  (`StaticMeshComponent.SetStaticMesh` (`self.TankTrack Left`) "/Game/Tank/tank_fbx_Track.tank_fbx_Track")
  (`StaticMeshComponent.SetStaticMesh` (`self.TankTrack Right`) "/Game/Tank/tank_fbx_Track.tank_fbx_Track")
  (`StaticMeshComponent.SetStaticMesh` (`self.TankTurret`) "/Game/Tank/tank_fbx_Turret.tank_fbx_Turret")
  (`PrimitiveComponent.SetPhysMaterialOverride` (`self.TankTrack Left`) "/Game/Tank/Track.Track")
  (`PrimitiveComponent.SetPhysMaterialOverride` (`self.TankTrack Right`) "/Game/Tank/Track.Track")
  (return))

(fn `UserConstructionScript`)